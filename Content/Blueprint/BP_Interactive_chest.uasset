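; BP_Interactive_chest is an interactive chest that opens and closes when interacted with.
; Interact alternates through a FlipFlop between playing the OpenChest timeline from the start and reversing it, with the timeline driving the pitch of the PivotEmpty component.
; On BeginPlay, SMChestTop takes the first material of SMBlock so the lid matches the block.
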(event `self.ReceiveBeginPlay`
  (`parent.ReceiveBeginPlay`)
  (`PrimitiveComponent.SetMaterial` (`self.SM_Chest_Top`) 0 (`PrimitiveComponent.GetMaterial` (`self.SM_Block`) 0)))

(event `self.Interact`
  (`/Engine/EditorBlueprintResources/StandardMacros.FlipFlop`
    (:`A`
      (bind (_direction _openchest) (`Timeline|OpenChest` :!via `PlayFromStart` :!label _label)
        (:`Update`
          (`SceneComponent.K2_SetRelativeRotation` (`self.PivotEmpty`) (`KismetMathLibrary.MakeRotator` 0.0 _openchest) false false))))
    (:`B`
      (goto _label :!via `Reverse`))))

(fn `UserConstructionScript`
  (`parent.UserConstructionScript`))