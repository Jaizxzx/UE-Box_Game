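; BP_Block is a block actor that can be destroyed over time, with the destruction cancellable before it completes.
; On BeginPlay it creates a dynamic material instance on its static mesh and sets the destroy timeline's play rate.
; StartDestroy plays the timeline from the start, driving the material's "Destroy Amount" parameter, and destroys the actor when finished.
; StopDestroy halts the timeline and resets that parameter.
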(event `self.ReceiveBeginPlay`
  (bind _sm_block (`self.SM_Block`))
  (bind _returnvalue (`PrimitiveComponent.CreateDynamicMaterialInstance` _sm_block 0 (`PrimitiveComponent.GetMaterial` _sm_block 0) "None"))
  (set `self.Block Mat` _returnvalue)
  (`TimelineComponent.SetPlayRate` (`self.destroy timeline`) (`self.Destroy Play Rate`)))

(event `Start Destroy`
  (bind (_direction _destroy_amount) (`Timeline|destroy timeline` :!via `PlayFromStart` :!label _label)
    (:`Update`
      (`MaterialInstanceDynamic.SetScalarParameterValue` (`self.Block Mat`) "Destroy Amount" _destroy_amount))
    (:`Finished`
      (`self.K2_DestroyActor`))))

(event `Stop Destroy`
  (`MaterialInstanceDynamic.SetScalarParameterValue` (`self.Block Mat`) "Destroy Amount" 0.0)
  (goto _label :!via `Stop`))

(fn `UserConstructionScript`)